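; MouseController is a cursor marker actor that follows the mouse's world position at the player character's height.
; Each tick, FFindMouseDirection traces under the cursor against one object type, and OffsetZ flattens the hit to the character's Z.
; The actor moves slightly below that point and yaws to face the player character.
; The helper also computes a yaw toward the cursor point, but Tick uses only its location.
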(event EventTick
  (params (DeltaSeconds :type Float%20%28single-precision%29))
  (Transformation|SetActorLocation (- (.Location (Math|Transform|BreakTransform (CallFunction|FFindMouseDirection))) "0, 0,8.000000") false false)
  (Transformation|SetActorRotation (Math|Rotator|MakeRotator 0.0 0.0 (.Yaw (Math|Rotator|BreakRotator (Math|Rotator|FindLookatRotation (Transformation|GetActorLocation) (Transformation|GetActorLocation (Game|GetPlayerCharacter 0))))))))

(fn ConstructionScript)

(fn OffsetZ
  (params (Vector :type Vector))
  (bind (_x _y) (Math|Vector|BreakVector Vector))
  (return (Math|Vector|MakeVector _x _y (.Z (Math|Vector|BreakVector (Transformation|GetActorLocation (Game|GetPlayerCharacter 0)))))))

(fn FFindMouseDirection
  (bind _returnvalue (Game|GetPlayerController 0))
  (bind _array (Utilities|Array|MakeArray "ObjectTypeQuery7"))
  (bind _hitresult (Class|PlayerController|GetHitResultUnderCursorforObjects _returnvalue _array true))
  (bind _location (Collision|BreakHitResult _hitresult))
  (bind _outvector (CallFunction|OffsetZ _location))
  (return (Math|Transform|MakeTransform _outvector (Math|Rotator|MakeRotator 0.0 0.0 (.Yaw (Math|Rotator|BreakRotator (Math|Rotator|FindLookatRotation (Transformation|GetActorLocation) _outvector)))))))