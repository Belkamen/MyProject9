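; Projectile actor that deals fixed damage to whatever it hits, credited to its Instigator, and expires after a few seconds.
; On BeginPlay its Sphere ignores the Instigator when moving, and a timed delay later stops and destroys it.
; On hit it applies damage, spawns a scaled impact effect and stops movement.
; A valid Head component is removed first, with a brief delay before the actor is destroyed.
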(event EventBeginPlay
  (Collision|IgnoreActorwhenMoving (Variables|Default|GetSphere) (Variables|Actor|GetInstigator) true)
  (Utilities|FlowControl|Delay 3.0)
  (Components|Movement|StopMovementImmediately (Variables|Default|GetProjectileMovement))
  (Actor|DestroyActor))

(event Collision|EventHit
  (params (MyComp :type Primitive%20Component%20Object%20Reference) (Other :type Actor%20Object%20Reference) (OtherComp :type Primitive%20Component%20Object%20Reference) (bSelfMoved :type Boolean) (HitLocation :type Vector :default "0, 0, 0") (HitNormal :type Vector :default "0, 0, 0") (NormalImpulse :type Vector :default "0, 0, 0") (Hit :type Hit%20Result%20Structure%20%28by%20ref%29))
  (bind _head (Variables|Default|GetHead))
  (Game|Damage|ApplyDamage Other 2.0 0 (Variables|Actor|GetInstigator))
  (bind _returnvalue (Niagara|SpawnSystematLocation "/Game/Assets/FX/Niagara_FX/FX_hit_impact.FX_hit_impact" (Transformation|GetActorLocation)))
  (Niagara|SetNiagaraVariable(Float) _returnvalue "Scale" 5.0)
  (Components|Movement|StopMovementImmediately (Variables|Default|GetProjectileMovement))
  (Utilities|IsValid _head
    (:Is%20Valid
      (Components|DestroyComponent _head)
      (Utilities|FlowControl|Delay 0.2))
    (:Is%20Not%20Valid
      _))
  (Actor|DestroyActor))

(fn ConstructionScript)