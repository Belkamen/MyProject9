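; Battlefield actor that stages a grid-based battle when Create_Battle is called with a list of enemy spawn cells.
; It adds the battle widget, blends the player's view to itself after a short delay, builds the field and hides its own mesh.
; CreateField spawns a grid of BF_Grid tiles around the actor, and SpawnActors puts player and enemy AI pawns on matching tile indices.
; An optional debug mode labels tiles with numbers colored by index band.
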(event Custom|Create_Battle
  (params (EnemySpawn :type Array%20of%20Integers))
  (bind _returnvalue (Game|GetPlayerController 0))
  (Variables|Index|SetEnemySpawn EnemySpawn)
  (bind _returnvalue_2 (UserInterface|CreateWidget "/Game/Blueprint/Battle_widget.Battle_widget_C" _returnvalue))
  (bind _output_get (Variables|Widget|SetBattleWidget _returnvalue_2))
  (UserInterface|Viewport|AddtoViewport _output_get 0)
  (Utilities|FlowControl|Delay 1.6)
  (Game|Player|SetViewTargetwithBlend _returnvalue self 0.0 "VTBlend_Linear" 0.0 false)
  (CallFunction|CreateField)
  (Rendering|SetVisibility (Variables|Default|GetStaticMesh) false false))

(event EventBeginPlay)

(fn ConstructionScript)

(fn CreateField
  (bind _worldgridsize (Variables|Size|GetWorldGridSize))
  (bind _worldgridsize_2 (Variables|Size|GetWorldGridSize))
  (Utilities|Array|Clear (Variables|Actor|GetGridArray))
  (Variables|Actor|SetWorldOffset (- (* (+ (Variables|Size|GetGridSize_X) _worldgridsize) 0.5) (* _worldgridsize 0.5)))
  (for _index (range 0 (- (Variables|Size|GetGridSize_X) 1))
    (for _index_2 (range 0 (- (Variables|Size|GetGridSize_Y) 1))
      (bind _returnvalue (Game|SpawnActorfromClass "/Game/Blueprint/Actors/BF_Grid.BF_Grid_C" (Math|Transform|MakeTransform (+ (Math|Vector|MakeVector (Math|Conversions|ToFloat(Integer) (- (* _index_2 _worldgridsize_2) (Math|Float|Truncate (Variables|Actor|GetWorldOffset)))) (Math|Conversions|ToFloat(Integer) (- (* _index _worldgridsize_2) (Math|Float|Truncate (Variables|Actor|GetWorldOffset)))) 0.0) (- (Transformation|GetActorLocation) (Math|Vector|MakeVector (* (- (Variables|Size|GetGridSize_Y) 1) 1e+02) (* (- (Variables|Size|GetGridSize_X) 1) 1e+02) 0.0)))) "AlwaysSpawn" 0 0))
      (bind _output_get (Variables|Actor|SetGrid _returnvalue))
      (bind _returnvalue_2 (Utilities|Array|AddUnique (Variables|Actor|GetGridArray) _output_get))
      (bind _output_get_2 (Variables|Index|SetInd _returnvalue_2))
      (if (Variables|Debug|GetbDebug?)
        (CallFunction|DebugGrid _output_get_2))
      (CallFunction|SpawnActors)))
  (return))

(fn DebugGrid
  (params (A :type Integer))
  (bind _returnvalue (+ A 1))
  (bind _grid (Variables|Actor|GetGrid))
  (if (> A 19)
    (if (> A 29)
      (Default|DebugText _grid _returnvalue "/Game/Assets/Materials/MI_GridRed.MI_GridRed")
      (else
        (Default|DebugText _grid _returnvalue "/Game/Assets/Materials/MI_GridGrey.MI_GridGrey")))
    (else
      (Default|DebugText _grid _returnvalue "/Game/Assets/Materials/MI_GridGreen.MI_GridGreen")))
  (return))

(fn SpawnActors
  (bind _ind (Variables|Index|GetInd))
  (bind _grid (Variables|Actor|GetGrid))
  (bind _returnvalue (Transformation|GetActorLocation _grid))
  (bind _returnvalue_2 (+ _returnvalue "0, 0,0.000000"))
  (for _array_element (Variables|Index|GetPlayerSpawn)
    (if (== _ind _array_element)
      (AI|SpawnAIFromClass "/Game/Blueprint/Main_Empty.Main_Empty_C" 0 _returnvalue_2 "0,90.000000, 0" true 0)))
  (for _array_element_2 (Variables|Index|GetEnemySpawn)
    (if (== _ind _array_element_2)
      (AI|SpawnAIFromClass "/Game/Blueprint/Enemy_Empty.Enemy_Empty_C" 0 _returnvalue_2 "0,-90.000000, 0" true 0)))
  (return))