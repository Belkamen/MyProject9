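; After-death dismemberment actor that breaks apart a destructible body and leaves blood decals where it hits.
; On BeginPlay it damages its Destructible component at the actor's location, with an impulse along the player character's forward vector.
; Sufficiently hard component hits spawn a long-lived, random blood decal aligned to the surface normal with random yaw.
; An unconnected loop for spawning random physics-simulated mesh pieces never runs.
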(event OnComponentHit(Destructible)
  (params (HitComponent :type Primitive%20Component%20Object%20Reference) (OtherActor :type Actor%20Object%20Reference) (OtherComp :type Primitive%20Component%20Object%20Reference) (NormalImpulse :type Vector :default "0, 0, 0") (Hit :type Hit%20Result%20Structure%20%28by%20ref%29))
  (bind (_bblockinghit _binitialoverlap _time _distance _location _impactpoint _normal) (Collision|BreakHitResult Hit))
  (bind _returnvalue (Math|Conversions|RotationFromXVector _normal))
  (bind (_roll _pitch) (Math|Rotator|BreakRotator _returnvalue))
  (if (> (Math|Vector|VectorLength NormalImpulse) 1e+02)
    (bind _returnvalue_2 (Rendering|Decal|SpawnDecalatLocation (Utilities|Select :Index (Math|Random|RandomInteger 6) :Option%200 "/Game/Assets/Textures/Blood/MI_D_Blood_01.MI_D_Blood_01" :Option%201 "/Game/Assets/Textures/Blood/MI_D_Blood_02.MI_D_Blood_02" :Option%202 "/Game/Assets/Textures/Blood/MI_D_Blood_04.MI_D_Blood_04" :Option%203 "/Game/Assets/Textures/Blood/MI_D_Blood_03.MI_D_Blood_03" :Option%204 "/Game/Assets/Textures/Blood/MI_D_Blood_05.MI_D_Blood_05" :Option%205 "/Game/Assets/Textures/Blood/MI_D_Blood_06.MI_D_Blood_06" :Option%206 "/Game/Assets/Textures/Blood/MI_D_Blood_07.MI_D_Blood_07") "50.000000,45.000000,45.000000" _location (Math|Rotator|MakeRotator _roll _pitch (Math|Random|RandomFloatinRange -9e+01 9e+01)) 1.5e+02))
    (Variables|Default|SetSpawn%20decal _returnvalue_2)))

(event EventBeginPlay
  (bind _returnvalue (Game|GetPlayerCharacter 0))
  (bind _returnvalue_2 (Transformation|GetActorForwardVector _returnvalue))
  (Class|DestructibleComponent|ApplyDamage (Variables|Default|GetDestructible) 15.0 (Transformation|GetActorLocation) (* _returnvalue_2 2.5e+02) (* (Math|Vector|VectorLength _returnvalue_2) 2e+03)))

(event Collision|EventHit
  (params (MyComp :type Primitive%20Component%20Object%20Reference) (Other :type Actor%20Object%20Reference) (OtherComp :type Primitive%20Component%20Object%20Reference) (bSelfMoved :type Boolean) (HitLocation :type Vector :default "0, 0, 0") (HitNormal :type Vector :default "0, 0, 0") (NormalImpulse :type Vector :default "0, 0, 0") (Hit :type Hit%20Result%20Structure%20%28by%20ref%29)))

(fn ConstructionScript
  (|CallParentFunction))