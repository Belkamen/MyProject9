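; BF_Grid is a grid cell actor that shows highlight and debug visuals and can spawn an AI pawn.
; Shortly after BeginPlay, it draws a debug sphere and turns its plane yellow if a sphere overlap finds pawns.
; Custom events toggle the highlight cube or spawn a Main_Empty AI at the cell.
; DebugText displays an integer value on the text render and reveals the plane with a supplied material.
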(event EventBeginPlay
  (bind _returnvalue (Transformation|GetActorLocation))
  (Utilities|FlowControl|Delay 0.2)
  (Rendering|Debug|DrawDebugSphere _returnvalue 1e+02 12 "(R=1.000000,G=1.000000,B=1.000000,A=1.000000)" 5.0 2.0)
  (bind _returnvalue_2 (Collision|SphereOverlapActors _returnvalue 1e+02 (Utilities|Array|MakeArray "ObjectTypeQuery3") 0))
  (if _returnvalue_2
    (Rendering|Material|SetMaterial (Variables|Default|GetPlane) 0 "/Game/Assets/Materials/MI_GridYelow.MI_GridYelow")))

(event EventBeginOverlapGrid
  (Rendering|SetVisibility (Variables|Default|GetCube) true false))

(event EventEndOverlapGrid
  (Rendering|SetVisibility (Variables|Default|GetCube) false false))

(event EventSpawnActor
  (AI|SpawnAIFromClass "/Game/Blueprint/Main_Empty.Main_Empty_C" 0 (Transformation|GetActorLocation) "0,90.000000, 0" true 0))

(fn ConstructionScript)

(fn DebugText
  (params (Value :type Integer%20%28by%20ref%29) (Material :type Material%20Interface%20Object%20Reference))
  (Variables|Default|SetValue Value)
  (Rendering|Components|TextRender|SetText (Variables|Default|GetTextRender) (Utilities|Text|ToText(Integer) Value))
  (Rendering|Material|SetMaterial (Variables|Default|GetPlane) 0 Material)
  (Rendering|SetVisibility (Variables|Default|GetPlane) true false)
  (return))