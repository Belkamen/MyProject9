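; Actor component that gives its owner health and hit feedback, destroying it when health runs out.
; The owner's damage event subtracts health, then spawns impact VFX, shakes the camera and emits blood toward the damager.
; Surviving hits briefly flash skeletal mesh materials through a TakeDamage parameter and apply timer-released hit stop, slowing owner and damager via CustomTimeDilation.
; Blood particle collisions spawn randomly sized and rotated decals aligned to the surface normal.
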(event Custom|GetHit
  (params (DamagedActor :type Actor%20Object%20Reference) (Damage :type Float%20%28single-precision%29) (DamageType :type Damage%20Type%20Object%20Reference) (InstigatedBy :type Controller%20Object%20Reference) (DamageCauser :type Actor%20Object%20Reference))
  (Variables|Default|SetDamager DamageCauser)
  (bind _output_get (Variables|Default|SetHealth (- (Variables|Default|GetHealth) Damage)))
  (CallFunction|EmitterSpawn)
  (CallFunction|FCameraShake)
  (CallFunction|BloodMechanic)
  (if (<= _output_get 0.0)
    (CallFunction|EndHitStop)
    (Actor|DestroyActor (Components|GetOwner))
    (else
      (CallFunction|StartTakeDamage)
      (CallFunction|StartHitStop "NewEnumerator0")
      (CallFunction|StartHitStop "NewEnumerator1"))))

(event Custom|EmitterSpawn
  (bind _returnvalue (Niagara|SpawnSystematLocation "/Game/Assets/FX/Niagara_FX/FX_hit_impact.FX_hit_impact" (Transformation|GetActorLocation (Components|GetOwner))))
  (Effects|Components|ParticleSystem|SetColorParameter _returnvalue "Color" "(R=1.000000,G=0.947105,B=0.364242,A=1.000000)")
  (Effects|Components|ParticleSystem|SetFloatParameter _returnvalue "Scale" 5.0))

(event EventBeginPlay
  (EventDispatchers|BindEventtoOnTakeAnyDamage (Components|GetOwner) (EventDispatchers|CreateEvent :!event Custom|GetHit)))

(fn StartHitStop
  (params (Enum_Hit :type Hit_Component_Owner%20Enum :default "NewEnumerator0"))
  (bind _damager (Variables|Default|GetDamager))
  (Utilities|IsValid _damager
    (:Is%20Valid
      (Variables|/Script/Engine.Actor|SetCustomTimeDilation (Utilities|Select :Index Enum_Hit :NewEnumerator0 (Components|GetOwner) :NewEnumerator1 _damager) 0.1)
      (Utilities|Time|SetTimerbyFunctionName 0 (Utilities|Select :Index Enum_Hit :NewEnumerator0 "End_HitStop_Owner" :NewEnumerator1 "End_HitStop") 0.09)
      (return))
    (:Is%20Not%20Valid
      (return))))

(fn EndHitStop
  (Variables|/Script/Engine.Actor|SetCustomTimeDilation (Variables|Default|GetDamager) 1.0)
  (return))

(fn EndHitStopOwner
  (Variables|/Script/Engine.Actor|SetCustomTimeDilation (Components|GetOwner) 1.0)
  (return))

(fn StartTakeDamage
  (bind _returnvalue (Components|GetOwner))
  (bind _returnvalue_2 (Actor|GetComponentbyClass _returnvalue "/Script/Engine.SkeletalMeshComponent"))
  (for (_array_element _array_index) (Rendering|Material|GetMaterials _returnvalue_2)
    (bind _returnvalue_3 (Rendering|Material|CreateDynamicMaterialInstance _returnvalue_2 _array_index _array_element "None" :!class /Script/Engine.PrimitiveComponent))
    (Rendering|Material|SetScalarParameterValue _returnvalue_3 "TakeDamage" 1.0 :!class /Script/Engine.MaterialInstanceDynamic))
  (Utilities|Time|SetTimerbyFunctionName 0 "End_TakeDamage" 0.2)
  (return))

(fn EndTakeDamage
  (bind _returnvalue (Components|GetOwner))
  (bind _returnvalue_2 (Actor|GetComponentbyClass _returnvalue "/Script/Engine.SkeletalMeshComponent"))
  (for (_array_element _array_index) (Rendering|Material|GetMaterials _returnvalue_2)
    (bind _returnvalue_3 (Rendering|Material|CreateDynamicMaterialInstance _returnvalue_2 _array_index _array_element "None" :!class /Script/Engine.PrimitiveComponent))
    (Rendering|Material|SetScalarParameterValue _returnvalue_3 "TakeDamage" 0.0 :!class /Script/Engine.MaterialInstanceDynamic))
  (return))

(fn FCameraShake
  (CameraShakes|StartCameraShake (Game|GetPlayerCameraManager 0) "/Game/Blueprints/HitShake.HitShake_C" 1.0 "CameraLocal" "0, 0, 0")
  (return))

(fn BloodMechanic
  (bind _returnvalue (Components|GetOwner))
  (bind _returnvalue_2 (Transformation|GetActorLocation _returnvalue))
  (bind _returnvalue_3 (Effects|SpawnEmitteratLocation "/Game/Assets/FX/BloodSplash.BloodSplash" _returnvalue_2 (Math|Rotator|FindLookatRotation _returnvalue_2 (Transformation|GetActorLocation (Variables|Default|GetDamager)))))
  (EventDispatchers|BindEventtoOnParticleCollide _returnvalue_3 (EventDispatchers|CreateEvent :!event HitComponentAutoGenFunc)))

(fn HitComponentAutoGenFunc
  (params (EventName :type Name) (EmitterTime :type Float%20%28single-precision%29) (ParticleTime :type Integer) (Location :type Vector) (Velocity :type Vector) (Direction :type Vector) (Normal :type Vector) (BoneName :type Name) (PhysMat :type Physical%20Material%20Object%20Reference))
  (bind _returnvalue (Math|Conversions|RotationFromXVector Normal))
  (bind _returnvalue_2 (Math|Random|RandomFloatinRange 64.0 128.0))
  (bind (_roll _pitch) (Math|Rotator|BreakRotator _returnvalue))
  (Rendering|Decal|SpawnDecalatLocation "/Game/Assets/Materials/MI_D_Blood_01.MI_D_Blood_01" (Math|Vector|MakeVector 5e+01 _returnvalue_2 _returnvalue_2) Location (Math|Rotator|MakeRotator _roll _pitch (Math|Random|RandomFloatinRange -9e+01 9e+01)) 1.5e+02)
  (return))