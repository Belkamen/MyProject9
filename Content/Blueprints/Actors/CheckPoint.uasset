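; CheckPoint is a trigger volume actor that detects the player character, with no save or respawn logic of its own.
; On box overlap, it casts the other actor to PlayerCharacter and only stores that reference.
; The construction script sizes the box from Size and applies a local offset of ZOffset vertically, also adding the box's current relative X and Y as horizontal offset.
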(event OnComponentBeginOverlap(Box)
  (params (OverlappedComponent :type Primitive%20Component%20Object%20Reference) (OtherActor :type Actor%20Object%20Reference) (OtherComp :type Primitive%20Component%20Object%20Reference) (OtherBodyIndex :type Integer) (bFromSweep :type Boolean) (SweepResult :type Hit%20Result%20Structure%20%28by%20ref%29))
  (bind _asplayer_character (Utilities|Casting|CastToPlayerCharacter OtherActor))
  (Variables|Default|SetAs%20Player%20Character _asplayer_character))

(fn ConstructionScript
  (bind _box (Variables|Default|GetBox))
  (bind _relativelocation (Variables|/Script/Engine.SceneComponent|GetRelativeLocation _box))
  (bind (_x _y) (Math|Vector|BreakVector _relativelocation))
  (Components|Box|SetBoxExtent _box (Variables|Default|GetSize) true)
  (Transformation|AddLocalOffset _box (Math|Vector|MakeVector _x _y (Variables|Default|GetZ_Offset)) false false))