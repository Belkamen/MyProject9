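; Post-death gore actor that shatters a destructible mesh and leaves blood where pieces land.
; On BeginPlay it picks one of two meshes at random, then damages it at the actor's location to fracture it, with impulse along the player character's forward vector.
; Sufficiently strong component hits spawn a long-lived blood decal oriented from the surface normal with randomized yaw.
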(event OnComponentHit(Destructible)
  (params (HitComponent :type Primitive%20Component%20Object%20Reference) (OtherActor :type Actor%20Object%20Reference) (OtherComp :type Primitive%20Component%20Object%20Reference) (NormalImpulse :type Vector :default "0, 0, 0") (Hit :type Hit%20Result%20Structure%20%28by%20ref%29))
  (bind (_bblockinghit _binitialoverlap _time _distance _location _impactpoint _normal) (Collision|BreakHitResult Hit))
  (bind _returnvalue (Math|Conversions|RotationFromXVector _normal))
  (bind (_roll _pitch) (Math|Rotator|BreakRotator _returnvalue))
  (if (> (Math|Vector|VectorLength NormalImpulse) 1e+02)
    (Rendering|Decal|SpawnDecalatLocation "/Game/Assets/Materials/MI_D_Blood_01.MI_D_Blood_01" "50.000000,45.000000,45.000000" _location (Math|Rotator|MakeRotator _roll _pitch (Math|Random|RandomFloatinRange -9e+01 9e+01)) 1.5e+02)))

(event EventBeginPlay
  (bind _returnvalue (Game|GetPlayerCharacter 0))
  (bind _returnvalue_2 (Transformation|GetActorForwardVector _returnvalue))
  (Class|DestructibleComponent|SetDestructibleMesh (Variables|Default|GetDestructible) (Utilities|Array|Get(acopy) (Variables|Default|GetMeshes) (Math|Random|RandomInteger 2)))
  (Class|DestructibleComponent|ApplyDamage (Variables|Default|GetDestructible) 15.0 (Transformation|GetActorLocation) (* _returnvalue_2 2.5e+02) (* (Math|Vector|VectorLength _returnvalue_2) 2e+03)))

(fn ConstructionScript
  (|CallParentFunction))